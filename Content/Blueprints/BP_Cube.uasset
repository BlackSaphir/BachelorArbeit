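; BP_Cube is an interactive cube actor that swaps its material and spawns an attached particle emitter when clicked or overlapped.
; The click interface event and the cube's overlap event both call ChangeMaterial behind an authority check, so only the server triggers the change.
; The overlap path also prints a "Hover" debug string, while the cursor-over event is empty.
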(event OnBeginCursorOver(Cube)
  (params (TouchedComponent :type Primitive%20Component%20Object%20Reference)))

(event OnComponentBeginOverlap(Cube)
  (params (OverlappedComponent :type Primitive%20Component%20Object%20Reference) (OtherActor :type Actor%20Object%20Reference) (OtherComp :type Primitive%20Component%20Object%20Reference) (OtherBodyIndex :type Integer) (bFromSweep :type Boolean) (SweepResult :type Hit%20Result%20Structure%20%28by%20ref%29))
  (Networking|SwitchHasAuthority
    (:Authority
      (Development|PrintString "Hover")
      (CallFunction|ChangeMaterial))))

(event Custom|Change%20Material
  (Rendering|Material|SetMaterial (Variables|Default|GetCube) 0 (Variables|Default|GetMaterial))
  (Effects|SpawnEmitterAttached 0 (Variables|Default|GetCube) "None"))

(event EventOnClickedInterface
  (Networking|SwitchHasAuthority
    (:Authority
      (CallFunction|ChangeMaterial))))

(fn ConstructionScript)