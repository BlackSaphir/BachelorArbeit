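; Game mode Blueprint that saves the current AR world map and publishes it for shared AR sessions.
; Save_AR_Map runs only when world mapping status is Mapped, saving the world asynchronously and checking the returned data.
; On authority, it sets the shared world data, converts the camera image to a PNG preview, then marks world sharing as ready.
; Debug prints report save progress and PNG conversion errors.
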(event Custom|Save_AR_Map
  (if (Utilities|Enum|Equal(Enum) (Class|ARBlueprintLibrary|GetWorldMappingStatus) "Mapped")
    (bind _savedworld (|ARSaveWorld)
      (:OnSuccess
        (Development|PrintString "Save success")
        (if (Utilities|Array|IsValidIndex _savedworld)
          (Development|PrintString "World valid")
          (Networking|SwitchHasAuthority
            (:Authority
              (Class|ARSharedWorldGameMode|SetARSharedWorldData _savedworld)
              (Development|PrintString "Set Shared World Data")
              (bind _returnvalue (Class|ARBlueprintLibrary|GetCameraImage))
              (bind _conversionresult (|ConverttoPNG _returnvalue true true 1.0 "None")
                (:OnSuccess
                  (Class|ARSharedWorldGameMode|SetPreviewImageData (.ImageData (Utilities|Struct|BreakAppleImageUtilsImageConversionResult _conversionresult)))
                  (Class|ARSharedWorldGameMode|SetARWorldSharingIsReady))
                (:OnFailure
                  (Development|PrintString (.Error (Utilities|Struct|BreakAppleImageUtilsImageConversionResult _conversionresult)))))))
          (else
            (Development|PrintString "World not valid")))))))

(fn ConstructionScript)